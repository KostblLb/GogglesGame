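; Traffic spawner actor that keeps adding cars to the world on a looping timer started at BeginPlay.
; SpawnCar creates a Car_Blueprint at the DefaultSceneRoot1 transform, rotates its mesh half a turn, then moves it to a random Y within a fixed band.
; A debug print re-rolls that random Y, so it may not match the car's position; SpawnRoadsign is an empty stub.
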(event `self.ReceiveBeginPlay`
  (`KismetSystemLibrary.K2_SetTimer` null "SpawnCar" 2.0 true))

(fn `SpawnCar`
  (bind _returnvalue (`KismetMathLibrary.MakeVector` (.x (`SceneComponent.K2_GetComponentLocation` (`self.DefaultSceneRoot1`))) (`KismetMathLibrary.RandomFloatInRange` -1000.0 1000.0) (.z (`SceneComponent.K2_GetComponentLocation` (`self.DefaultSceneRoot1`)))))
  (bind _returnvalue_2 (`|SpawnActorFromClass` "/Game/GogglesGameContent/Blueprints/car_Blueprint.car_Blueprint_C" (`SceneComponent.K2_GetComponentToWorld` (`self.DefaultSceneRoot1`)) "Undefined" "OverrideRootScale" null null))
  (`SceneComponent.K2_SetWorldRotation` (`StaticMeshActor.StaticMeshComponent` _returnvalue_2) (struct :`Yaw` 180.0) false false)
  (`self.K2_SetActorRelativeLocation` _returnvalue_2 _returnvalue false false)
  (`KismetSystemLibrary.PrintString` (`KismetStringLibrary.Conv_VectorToString` _returnvalue)))

(fn `SpawnRoadsign`)

(fn `UserConstructionScript`)